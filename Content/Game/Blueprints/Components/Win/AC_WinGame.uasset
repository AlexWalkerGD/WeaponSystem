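; Actor component that handles the win condition: the game is won when every BaseEnemy is dead.
; On BeginPlay it binds an event to each enemy's death notification.
; IsGameOver scans all enemies and clears a flag if any is still alive.
; If the flag holds, it stops the owner's weapon fire, shows the W_Winner widget and switches to UI-only input with a visible cursor.
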(event EventBeginPlay
  (bind _outactors (Actor|GetAllActorsOfClass "/Game/Game/Blueprints/Characters/Enemy/BaseEnemy.BaseEnemy_C"))
  (for _array_element _outactors
    (EventDispatchers|BindEventtoDeadEnemy _array_element (EventDispatchers|CreateEvent :!event IsGameOver?))))

(fn IsGameOver?
  (bind _returnvalue (Game|GetPlayerController 0))
  (bind _outactors (Actor|GetAllActorsOfClass "/Game/Game/Blueprints/Characters/Enemy/BaseEnemy.BaseEnemy_C"))
  (for _array_element _outactors
    (if (not (Variables|/Game/Game/Blueprints/Characters/Enemy/BaseEnemy.BaseEnemy_C|GetDead _array_element))
      (LocalVariables|SetIsOverGame false)))
  (if (LocalVariables|GetIsOverGame)
    (Default|StopFire (CallFunction|FindWeaponComponent (Components|GetOwner)))
    (bind _returnvalue_2 (UserInterface|CreateWidget "/Game/Game/UI/W_Winner.W_Winner_C"))
    (UserInterface|Viewport|AddtoViewport _returnvalue_2 0)
    (Input|SetInputModeUIOnly _returnvalue _returnvalue_2 "DoNotLock" false)
    (Variables|/Script/Engine.PlayerController|SetbShowMouseCursor _returnvalue true)))