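; Actor component that holds a character's replicated inventory of weapons and ammo for pickup, firing and reloading.
; Ammo pickups stack by type up to a cap and return leftovers; weapon pickups swap a same-named weapon, handing back the old one, or append.
; Firing decrements clip ammo; reloading moves available reserve into the clip, removing emptied ammo entries.
; OnRep functions broadcast list and weapon-type updates; last-changed indices are tracked.
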(event EventBeginPlay)

(event EventTick
  (params (DeltaSeconds :type Float%20%28single-precision%29)))

(fn TryCollectAmmo
  (params (AmmoInfo :type PDA%20Ammo%20Info%20Object%20Reference) (AmmoAmount :type Integer))
  (bind _output_get (LocalVariables|SetTemporayArray (Variables|Private|Ammo|GetAmmo)))
  (bind (_array_element _array_index) (Utilities|Array|ForEachLoopwithBreak _output_get :!label _label)
    (:LoopBody
      (LocalVariables|SetArrayIndex _array_index)
      (if (Utilities|Enum|Equal(Enum) (Variables|/Game/Game/Blueprints/Itens/Data/PrimaryDataAssets/PDA_AmmoInfo.PDA_AmmoInfo_C|GetAmmoType (Utilities|Struct|BreakST_Ammo _array_element)) (Variables|/Game/Game/Blueprints/Itens/Data/PrimaryDataAssets/PDA_AmmoInfo.PDA_AmmoInfo_C|GetAmmoType AmmoInfo))
        (LocalVariables|SetFoundAmmo true)
        (Utilities|FlowControl|Sequence
          (:then_0
            (goto _label Break))
          (:then_1
            (bind (_allammoadded _ammoreimaining) (Private|Ammo|IncreaseAmmo (LocalVariables|GetTemporayArray) (LocalVariables|GetArrayIndex) AmmoAmount))
            (return _allammoadded _ammoreimaining)))))
    (:Completed
      (if (not (LocalVariables|GetFoundAmmo))
        (bind _returnvalue (Utilities|Array|Add (LocalVariables|GetTemporayArray) (Utilities|Struct|MakeST_Ammo AmmoInfo)))
        (LocalVariables|SetArrayIndex _returnvalue)
        (bind (_allammoadded_2 _ammoreimaining_2) (Private|Ammo|IncreaseAmmo (LocalVariables|GetTemporayArray) (LocalVariables|GetArrayIndex) AmmoAmount))
        (return _allammoadded_2 _ammoreimaining_2)))))

(fn IncreaseAmmo
  (params (AmmoStruct :type Array%20of%20ST%20Ammo%20Structures) (ArrayIndex :type Integer) (AmmoToIncrease :type Integer))
  (LocalVariables|SetTemporaryArray AmmoStruct)
  (LocalVariables|SetPDAAmmoInfo (.AmmoInfo (Utilities|Struct|BreakST_Ammo (Utilities|Array|Get(acopy) (LocalVariables|GetTemporaryArray) ArrayIndex))))
  (if (> (Variables|/Game/Game/Blueprints/Itens/Data/PrimaryDataAssets/PDA_AmmoInfo.PDA_AmmoInfo_C|GetMaxAmmoAllowed (.AmmoInfo (Utilities|Struct|BreakST_Ammo (Utilities|Array|Get(acopy) (LocalVariables|GetTemporaryArray) ArrayIndex)))) (.AmmoAmount (Utilities|Struct|BreakST_Ammo (Utilities|Array|Get(acopy) (LocalVariables|GetTemporaryArray) ArrayIndex))))
    (Variables|Private|Ammo|SetLastIndexAmmoArray ArrayIndex)
    (LocalVariables|SetLocalAmmoRemaining (- (+ (.AmmoAmount (Utilities|Struct|BreakST_Ammo (Utilities|Array|Get(acopy) (LocalVariables|GetTemporaryArray) ArrayIndex))) AmmoToIncrease) (Math|Integer|Clamp(Integer) (+ (.AmmoAmount (Utilities|Struct|BreakST_Ammo (Utilities|Array|Get(acopy) (LocalVariables|GetTemporaryArray) ArrayIndex))) AmmoToIncrease) 0 (Variables|/Game/Game/Blueprints/Itens/Data/PrimaryDataAssets/PDA_AmmoInfo.PDA_AmmoInfo_C|GetMaxAmmoAllowed (.AmmoInfo (Utilities|Struct|BreakST_Ammo (Utilities|Array|Get(acopy) (LocalVariables|GetTemporaryArray) ArrayIndex)))))))
    (Utilities|Array|SetArrayElem (LocalVariables|GetTemporaryArray) ArrayIndex (Utilities|Struct|MakeST_Ammo (.AmmoInfo (Utilities|Struct|BreakST_Ammo (Utilities|Array|Get(acopy) (LocalVariables|GetTemporaryArray) ArrayIndex))) (Math|Integer|Clamp(Integer) (+ (.AmmoAmount (Utilities|Struct|BreakST_Ammo (Utilities|Array|Get(acopy) (LocalVariables|GetTemporaryArray) ArrayIndex))) AmmoToIncrease) 0 (Variables|/Game/Game/Blueprints/Itens/Data/PrimaryDataAssets/PDA_AmmoInfo.PDA_AmmoInfo_C|GetMaxAmmoAllowed (.AmmoInfo (Utilities|Struct|BreakST_Ammo (Utilities|Array|Get(acopy) (LocalVariables|GetTemporaryArray) ArrayIndex)))))))
    (Variables|Private|Ammo|SetAmmo (LocalVariables|GetTemporaryArray))
    (return (not (> (LocalVariables|GetLocalAmmoRemaining) 0)) (LocalVariables|GetLocalAmmoRemaining))
    (else
      (return false AmmoToIncrease))))

(fn OnRepAmmo
  (Default|CallAmmoListUpdate self))

(fn GetAmmoList
  (return (Variables|Private|Ammo|GetAmmo)))

(fn TryCollectWeapon
  (params (WeaponInfo :type PDA%20Weapon%20Info%20Object%20Reference) (ClipAmmoAmount :type Integer) (WeaponType :type BP%20Weapon%20Pickup%20Object%20Reference))
  (bind _output_get (LocalVariables|SetLocalWeaponArray (Variables|Private|Weapon|GetWeapon)))
  (bind (_array_element _array_index) (Utilities|Array|ForEachLoopwithBreak _output_get :!label _label)
    (:LoopBody
      (if (Utilities|Enum|Equal(Enum) (Variables|/Game/Game/Blueprints/Itens/Data/PrimaryDataAssets/PDA_WeaponInfo.PDA_WeaponInfo_C|GetWeaponName (Utilities|Struct|BreakST_Weapon _array_element)) (Variables|/Game/Game/Blueprints/Itens/Data/PrimaryDataAssets/PDA_WeaponInfo.PDA_WeaponInfo_C|GetWeaponName WeaponInfo))
        (Variables|Private|Weapon|SetLastIndexWeaponArray _array_index)
        (LocalVariables|SetWeaponTypeFound true)
        (Utilities|FlowControl|Sequence
          (:then_0
            (goto _label Break))
          (:then_1
            (LocalVariables|SetNewWeaponSwap (.WeaponInfo (Utilities|Struct|BreakST_Weapon (Utilities|Array|Get(acopy) (LocalVariables|GetLocalWeaponArray) (Variables|Private|Weapon|GetLastIndexWeaponArray)))))
            (LocalVariables|SetNewClipAmmoAmount (.ClipAmmo (Utilities|Struct|BreakST_Weapon (Utilities|Array|Get(acopy) (LocalVariables|GetLocalWeaponArray) (Variables|Private|Weapon|GetLastIndexWeaponArray)))))
            (Utilities|Array|SetArrayElem (LocalVariables|GetLocalWeaponArray) (Variables|Private|Weapon|GetLastIndexWeaponArray) (Utilities|Struct|MakeST_Weapon WeaponInfo ClipAmmoAmount))
            (Variables|Default|SetWeapon%20Types WeaponType)
            (Variables|Private|Weapon|SetWeapon (LocalVariables|GetLocalWeaponArray))
            (return true (LocalVariables|GetNewWeaponSwap) (LocalVariables|GetNewClipAmmoAmount))))))
    (:Completed
      (if (LocalVariables|GetWeaponTypeFound)
        (Development|PrintString "Hello" true true "(R=0.235476,G=0.000000,B=0.572917,A=1.000000)")
        (else
          (Development|PrintString "Hello" true true "(R=0.178845,G=1.000000,B=0.000000,A=1.000000)")
          (Utilities|FlowControl|Sequence
            (:then_0
              (if (Utilities|Array|IsEmpty (LocalVariables|GetLocalWeaponArray))
                (Default|CallFirstWeaponAdded)))
            (:then_1
              (bind _returnvalue (Utilities|Array|Add (LocalVariables|GetLocalWeaponArray) (Utilities|Struct|MakeST_Weapon WeaponInfo ClipAmmoAmount)))
              (Variables|Private|Weapon|SetLastIndexWeaponArray _returnvalue)
              (Variables|Default|SetWeapon%20Types WeaponType)
              (Variables|Private|Weapon|SetWeapon (LocalVariables|GetLocalWeaponArray))
              (return false 0 0))))))))

(fn OnRepWeapon
  (Default|CallWeaponListUpdate self))

(fn GetWeaponList
  (return (Variables|Private|Weapon|GetWeapon)))

(fn GetLastAmmoIndex
  (return (Variables|Private|Ammo|GetLastIndexAmmoArray)))

(fn GetLastWeaponIndex
  (return (Variables|Private|Weapon|GetLastIndexWeaponArray)))

(fn TrytoConsumeWeaponAmmo
  (params (CurrentWeaponIndex :type Integer))
  (LocalVariables|SetLocalWeaponList (Variables|Private|Weapon|GetWeapon))
  (if (> (Utilities|Struct|BreakST_Weapon (Utilities|Array|Get(acopy) (LocalVariables|GetLocalWeaponList) CurrentWeaponIndex)) 0)
    (Utilities|Array|SetArrayElem (LocalVariables|GetLocalWeaponList) CurrentWeaponIndex (Utilities|Struct|MakeST_Weapon (.WeaponInfo (Utilities|Struct|BreakST_Weapon (Utilities|Array|Get(acopy) (LocalVariables|GetLocalWeaponList) CurrentWeaponIndex))) (- (.ClipAmmo (Utilities|Struct|BreakST_Weapon (Utilities|Array|Get(acopy) (LocalVariables|GetLocalWeaponList) CurrentWeaponIndex))) 1)))
    (Variables|Private|Weapon|SetLastIndexWeaponArray CurrentWeaponIndex)
    (Variables|Private|Weapon|SetWeapon (LocalVariables|GetLocalWeaponList))
    (return true)
    (else
      (return false))))

(fn TrytoAddAmmotoClipWeapon
  (params (CurrentWeaponIndex :type Integer) (CurrentAmmoIndex :type Integer))
  (if (Utilities|Array|IsValidIndex (Variables|Private|Ammo|GetAmmo) CurrentAmmoIndex)
    (LocalVariables|SetLocalWeaponList (Variables|Private|Weapon|GetWeapon))
    (LocalVariables|SetLocalAmmoList (Variables|Private|Ammo|GetAmmo))
    (if (> (Utilities|Struct|BreakST_Ammo (Utilities|Array|Get(acopy) (LocalVariables|GetLocalAmmoList) CurrentAmmoIndex)) 0)
      (LocalVariables|SetWeaponAmmoNeeded (- (Variables|/Game/Game/Blueprints/Itens/Data/PrimaryDataAssets/PDA_WeaponInfo.PDA_WeaponInfo_C|GetMaxClipAmmo (.WeaponInfo (Utilities|Struct|BreakST_Weapon (Utilities|Array|Get(acopy) (LocalVariables|GetLocalWeaponList) CurrentWeaponIndex)))) (.ClipAmmo (Utilities|Struct|BreakST_Weapon (Utilities|Array|Get(acopy) (LocalVariables|GetLocalWeaponList) CurrentWeaponIndex)))))
      (bind _clipammotoincrease (CallFunction|FindAvailableAmmo (LocalVariables|GetWeaponAmmoNeeded) CurrentAmmoIndex))
      (LocalVariables|SetClipAmmoToIncrease _clipammotoincrease)
      (CallFunction|DecreaseAmmo (LocalVariables|GetLocalAmmoList) CurrentAmmoIndex (LocalVariables|GetClipAmmoToIncrease))
      (CallFunction|IncreaseClipAmmo (LocalVariables|GetLocalWeaponList) CurrentWeaponIndex (LocalVariables|GetClipAmmoToIncrease))
      (return true)
      (else
        (return false)))
    (else
      (return false))))

(fn FindAvailableAmmo
  (params (WeaponAmmoNeeded :type Integer) (CurrentAmmoIndex :type Integer))
  (LocalVariables|SetInventoryAmmo (Utilities|Struct|BreakST_Ammo (Utilities|Array|Get(acopy) (Variables|Private|Ammo|GetAmmo) CurrentAmmoIndex)))
  (if (>= (LocalVariables|GetInventoryAmmo) WeaponAmmoNeeded)
    (return WeaponAmmoNeeded)
    (else
      (return (LocalVariables|GetInventoryAmmo)))))

(fn DecreaseAmmo
  (params (AmmoStruct :type Array%20of%20ST%20Ammo%20Structures) (ArrayIndex :type Integer) (AmmoToDecrease :type Integer))
  (bind _output (Utilities|Array|Get(acopy) AmmoStruct ArrayIndex))
  (bind (_ammoinfo _ammoamount) (Utilities|Struct|BreakST_Ammo _output))
  (bind _returnvalue (- _ammoamount AmmoToDecrease))
  (if (> _returnvalue 0)
    (Utilities|Array|SetArrayElem AmmoStruct ArrayIndex (Utilities|Struct|MakeST_Ammo _ammoinfo _returnvalue))
    (Variables|Private|Ammo|SetLastIndexAmmoArray ArrayIndex)
    (Variables|Private|Ammo|SetAmmo AmmoStruct)
    (else
      (Utilities|Array|RemoveIndex AmmoStruct ArrayIndex)
      (Variables|Private|Ammo|SetLastIndexAmmoArray -1)
      (Variables|Private|Ammo|SetAmmo AmmoStruct))))

(fn IncreaseClipAmmo
  (params (WeaponStruct :type Array%20of%20ST%20Weapon%20Structures) (Array%20Index :type Integer) (AmmoToIncrease :type Integer))
  (bind _output (Utilities|Array|Get(acopy) WeaponStruct Array%20Index))
  (bind (_weaponinfo _clipammo) (Utilities|Struct|BreakST_Weapon _output))
  (Utilities|Array|SetArrayElem WeaponStruct Array%20Index (Utilities|Struct|MakeST_Weapon _weaponinfo (+ _clipammo AmmoToIncrease)))
  (Variables|Private|Weapon|SetLastIndexWeaponArray Array%20Index)
  (Variables|Private|Weapon|SetWeapon WeaponStruct))

(fn OnRepWeaponTypes
  (Default|CallWeaponTypeUpdate (Variables|Default|GetWeapon%20Types) self))