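; Base enemy Blueprint with replicated health that ragdolls when that health runs out.
; AnyDamage subtracts from Health with clamping, then switches the mesh to the Ragdoll collision profile and enables physics simulation at zero.
; BeginPlay and OnRep_Health show rounded Health on a widget component, reusing the W3D_AmmoNumber widget's UpdateAmmo as the health readout.
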(event EventBeginPlay
  (bind _asw3d_ammo_number (Utilities|Casting|CastToW3D_AmmoNumber (UserInterface|GetWidget (Variables|Default|GetWidget))))
  (Default|UpdateAmmo _asw3d_ammo_number (Math|Float|Round (Variables|Default|GetHealth))))

(event Collision|EventActorBeginOverlap
  (params (OtherActor :type Actor%20Object%20Reference)))

(event EventTick
  (params (DeltaSeconds :type Float%20%28single-precision%29)))

(event Game|Damage|EventAnyDamage
  (params (Damage :type Float%20%28single-precision%29) (DamageType :type Damage%20Type%20Object%20Reference) (InstigatedBy :type Controller%20Object%20Reference) (DamageCauser :type Actor%20Object%20Reference))
  (bind _mesh (Variables|Character|GetMesh))
  (Variables|Default|SetHealth (Math|Float|Clamp(Float) (- (Variables|Default|GetHealth) Damage) 0.0 1e+02))
  (if (== (Variables|Default|GetHealth) 0.0)
    (Collision|SetCollisionProfileName _mesh "Ragdoll" false :!class /Script/Engine.PrimitiveComponent)
    (Physics|SetSimulatePhysics _mesh true)))

(fn ConstructionScript)

(fn OnRepHealth
  (bind _asw3d_ammo_number (Utilities|Casting|CastToW3D_AmmoNumber (UserInterface|GetWidget (Variables|Default|GetWidget))))
  (Default|UpdateAmmo _asw3d_ammo_number (Math|Float|Round (Variables|Default|GetHealth))))