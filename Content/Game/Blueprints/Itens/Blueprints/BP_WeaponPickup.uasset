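; Weapon pickup actor that hands a weapon and its clip ammo to an inventory component on collection.
; If the inventory swaps weapons, the pickup takes on the swapped-out weapon and ammo and stays uncollected.
; Construction creates dynamic materials tinted by rarity and flagged as pickup, while a ping-pong timeline floats the mesh.
; A widget shows clip ammo, refreshed on BeginPlay and through its OnRep.
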(event Custom|Reverse
  (bind _floating (Timeline|Floating ReverseFromEnd)
    (:Update
      (Transformation|SetRelativeLocation (Variables|Default|GetSkeletalMesh) _floating false false))
    (:Finished
      (Utilities|FlowControl|FlipFlop
        (:A
          (CallFunction|Reverse))
        (:B
          (CallFunction|Play))))))

(event Custom|Play
  (bind _floating (Timeline|Floating PlayFromStart)
    (:Update
      (Transformation|SetRelativeLocation (Variables|Default|GetSkeletalMesh) _floating false false))
    (:Finished
      (Utilities|FlowControl|FlipFlop
        (:A
          (CallFunction|Reverse))
        (:B
          (CallFunction|Play))))))

(event EventBeginPlay
  (|CallParentFunction)
  (CallFunction|UpdateLocalWidget)
  (bind _floating (Timeline|Floating Play)
    (:Update
      (Transformation|SetRelativeLocation (Variables|Default|GetSkeletalMesh) _floating false false))
    (:Finished
      (Utilities|FlowControl|FlipFlop
        (:A
          (CallFunction|Reverse))
        (:B
          (CallFunction|Play))))))

(fn ConstructionScript
  (|CallParentFunction)
  (CallFunction|SetTypeWeapon))

(fn RequestCollectItem
  (params (InventoryComponent :type AC%20Inventory%20Component%20Object%20Reference))
  (bind _aspda_weapon_info (Utilities|Casting|CastToPDA_WeaponInfo (Variables|Default|GetItemInfo))
    (:then
      (bind (_swapweapon _weapontoswap _clipammotoswap) (Default|TryCollectWeapon InventoryComponent _aspda_weapon_info (Variables|Default|GetClipAmmoAmount) self))
      (if _swapweapon
        ;[0 0.6447 1 0] Refresh the  to new weapon to pickup
        (Variables|Default|SetItemInfo _weapontoswap)
        (Variables|Default|SetClipAmmoAmount _clipammotoswap)
        (return false)
        (else
          (return true))))
    (:CastFailed
      (return false))))

(fn OnRepClipAmmoAmount
  (CallFunction|UpdateLocalWidget))

(fn UpdateLocalWidget
  (bind _asw3d_ammo_number (Utilities|Casting|CastToW3D_AmmoNumber (UserInterface|GetWidget (Variables|Default|GetWidget))))
  (Default|UpdateAmmo _asw3d_ammo_number (Variables|Default|GetClipAmmoAmount)))

(fn SetTypeWeapon
  (bind _st_typeweapon (Variables|Default|GetST_TypeWeapon))
  (for (_array_element _array_index) (Rendering|Material|GetMaterials (Variables|Default|GetSkeletalMesh))
    (bind _returnvalue (Rendering|Material|CreateDynamicMaterialInstance _array_element "None" "None" :!class /Script/Engine.KismetMaterialLibrary))
    (Rendering|Material|SetMaterial (Variables|Default|GetSkeletalMesh) _array_index _returnvalue)
    (Rendering|Material|SetVectorParameterValue _returnvalue "Color" (Utilities|Select :Index (Variables|Default|GetE_Type) :NewEnumerator0 (.normal _st_typeweapon) :NewEnumerator1 (.rare _st_typeweapon) :NewEnumerator2 (.mystic _st_typeweapon) :NewEnumerator3 (.epic _st_typeweapon)) :!class /Script/Engine.MaterialInstanceDynamic)
    (Rendering|Material|SetScalarParameterValue _returnvalue "IsPickup" 1.0 :!class /Script/Engine.MaterialInstanceDynamic)))