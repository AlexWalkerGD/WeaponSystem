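; BP_AmmoPickup is an ammo pickup item that offers its ammo to the collector's inventory component.
; RequestCollectItem casts ItemInfo to PDA_AmmoInfo, calls TryCollectAmmo with the current amount, then resets AmmoAmount to 20 and always returns false.
; BeginPlay and the AmmoAmount OnRep both call UpdateLocalWidget, which is empty here.
; A RespawnAmmo call exists but is unconnected.
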(event EventBeginPlay
  (|CallParentFunction)
  (CallFunction|UpdateLocalWidget))

(fn ConstructionScript
  (|CallParentFunction))

(fn RequestCollectItem
  (params (InventoryComponent :type AC%20Inventory%20Component%20Object%20Reference))
  (bind _aspda_ammo_info (Utilities|Casting|CastToPDA_AmmoInfo (Variables|Default|GetItemInfo))
    (:then
      (Default|TryCollectAmmo InventoryComponent _aspda_ammo_info (Variables|Default|GetAmmoAmount))
      (Variables|Default|SetAmmoAmount 20)
      (return false))
    (:CastFailed
      (return false))))

(fn OnRepAmmoAmount
  (CallFunction|UpdateLocalWidget))

(fn UpdateLocalWidget)