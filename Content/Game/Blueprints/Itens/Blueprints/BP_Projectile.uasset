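; BP_Projectile is a weapon projectile that damages Enemy-tagged actors overlapping its sphere and can hit several in succession.
; It skips the last actor hit and stops dealing damage at the current weapon's hit limit.
; Damage starts from the weapon's value, decays exponentially per previous hit, and scales by hit-bone name substrings favoring head, then torso, then other bones.
; Each hit also prints the bone name.
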(event OnComponentBeginOverlap(Sphere)
  (params (OverlappedComponent :type Primitive%20Component%20Object%20Reference) (OtherActor :type Actor%20Object%20Reference) (OtherComp :type Primitive%20Component%20Object%20Reference) (OtherBodyIndex :type Integer) (bFromSweep :type Boolean) (SweepResult :type Hit%20Result%20Structure%20%28by%20ref%29))
  (bind _currentweapon (Variables|Default|GetCurrentWeapon))
  (bind _weaponinfo (Utilities|Struct|BreakST_Weapon _currentweapon))
  (if (and (Actor|ActorHasTag OtherActor "Enemy") (!= OtherActor (Variables|Default|GetHitActor)))
    (Variables|Default|SetHitActor OtherActor)
    (if (< (Variables|Default|GetHits) (Variables|/Game/Game/Blueprints/Itens/Data/PrimaryDataAssets/PDA_WeaponInfo.PDA_WeaponInfo_C|GetMaxHitAllowed (.WeaponInfo (Utilities|Struct|BreakST_Weapon (Variables|Default|GetCurrentWeapon)))))
      (Development|PrintString (Utilities|String|ToString(Name) (.hitbonename SweepResult)))
      (Game|Damage|ApplyDamage (Variables|Default|GetHitActor) (* (CallFunction|GetDamageMultiplierbyBone (.hitbonename SweepResult)) (* (Variables|/Game/Game/Blueprints/Itens/Data/PrimaryDataAssets/PDA_WeaponInfo.PDA_WeaponInfo_C|GetDamage _weaponinfo) (Math|Float|Power (- 1.0 (Variables|/Game/Game/Blueprints/Itens/Data/PrimaryDataAssets/PDA_WeaponInfo.PDA_WeaponInfo_C|GetLostDamagePercent _weaponinfo)) (Math|Conversions|ToFloat(Integer) (Variables|Default|GetHits))))) 0 0)
      (Math|Integer|IncrementInt (Variables|Default|GetHits)))))

(event EventBeginPlay)

(fn ConstructionScript)

(fn GetDamageMultiplierbyBone
  (params (HitBone :type Name))
  (bind _returnvalue (Utilities|String|ToString(Name) HitBone))
  (if (Utilities|String|Contains _returnvalue "head")
    (return 1.0)
    (elif (Math|Boolean|ORBoolean (Utilities|String|Contains _returnvalue "pelvis") (Utilities|String|Contains _returnvalue "clavicle") (Utilities|String|Contains _returnvalue "spine"))
      (return 0.6)
      (elif (or (Utilities|String|Contains _returnvalue "_r") (Utilities|String|Contains _returnvalue "_l"))
        (return 0.4)
        (else
          (return 0.4))))))